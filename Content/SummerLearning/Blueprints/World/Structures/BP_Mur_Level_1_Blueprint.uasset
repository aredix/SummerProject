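; BP_Mur_Level_1_Blueprint is a wall with square and rectangle passages that gate the player by shape.
; On overlap with either verification box, it casts the actor to BP_BasePlayer and checks its Status enum.
; A matching status disables collision on that passage's blocking box; any other status restores query and physics collision.
; Collision changes only on begin overlap, so each passage keeps its last state until the next check.
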(event `self.CB_Verif_Shape_Rectangle.OnComponentBeginOverlap`
  (params (OverlappedComponent :type "PrimitiveComponent Object Reference") (OtherActor :type "Actor Object Reference") (OtherComp :type "PrimitiveComponent Object Reference") (OtherBodyIndex :type Integer) (bFromSweep :type Boolean) (SweepResult :type "HitResult Structure (by ref)"))
  (bind _cb_passage_rectangle (`self.CB_Passage_Rectangle`))
  (bind _asbp_base_player (cast `/Game/SummerLearning/Blueprints/Player/BP_BasePlayer` OtherActor))
  (if (`|EnumEquality` (`/Game/SummerLearning/Blueprints/Player/BP_BasePlayer.Status` _asbp_base_player) "NewEnumerator1")
    (`PrimitiveComponent.SetCollisionEnabled` _cb_passage_rectangle "NoCollision")
    (else
      (`PrimitiveComponent.SetCollisionEnabled` _cb_passage_rectangle "QueryAndPhysics"))))

(event `self.CB_Verif_Shape_Carré.OnComponentBeginOverlap`
  (params (OverlappedComponent :type "PrimitiveComponent Object Reference") (OtherActor :type "Actor Object Reference") (OtherComp :type "PrimitiveComponent Object Reference") (OtherBodyIndex :type Integer) (bFromSweep :type Boolean) (SweepResult :type "HitResult Structure (by ref)"))
  (bind `_cb_passage_carré` (`self.CB_Passage_Carré`))
  (bind _asbp_base_player (cast `/Game/SummerLearning/Blueprints/Player/BP_BasePlayer` OtherActor))
  (if (`|EnumEquality` (`/Game/SummerLearning/Blueprints/Player/BP_BasePlayer.Status` _asbp_base_player) "NewEnumerator0")
    (`PrimitiveComponent.SetCollisionEnabled` `_cb_passage_carré` "NoCollision")
    (else
      (`PrimitiveComponent.SetCollisionEnabled` `_cb_passage_carré` "QueryAndPhysics"))))

(fn `UserConstructionScript`)