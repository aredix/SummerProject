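; Dialogue component for the World 4 ending NPC: Laura congratulates the player in French on completing the trials, recaps color mixing and says goodbye.
; Its Dialogue function calls the parent version, then increments the main dialogue counter (CompteurDialoguePrincipal) on BP_BasePlayer.
; It then plays a linear chain of AddDialogue lines, each with a single continue option, and closes the conversation after the last.
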(fn `Dialogue`
  (`parent.Dialogue`)
  (bind _asbp_base_player (cast `/Game/SummerLearning/Blueprints/Player/BP_BasePlayer` (`GameplayStatics.GetPlayerPawn` 0)))
  (`/Engine/EditorBlueprintResources/StandardMacros.IncrementInt` (`/Game/SummerLearning/Blueprints/Player/BP_BasePlayer.CompteurDialoguePrincipal` _asbp_base_player)
    (:`  `
      (bind _state (`self.AddDialogue` "Laura" "Bravo tu as réussi à compléter toutes les épreuves." (`|MakeArray` "Continuer" :!type "Text")))
      (switch `/Game/SummerLearning/Blueprints/Dialogue/Enum_DialogueState` _state
        (:`NewEnumerator0`
          (bind _state_2 (`self.AddDialogue` "Laura" "Maintenant, il faut savoir qu'il existe une infinité de couleur." (`|MakeArray` "Continuer" :!type "Text")))
          (switch `/Game/SummerLearning/Blueprints/Dialogue/Enum_DialogueState` _state_2
            (:`NewEnumerator0`
              (bind _state_3 (`self.AddDialogue` "Laura" "Aujourd'hui on a vu que mélanger deux couleurs une troisième couleur." (`|MakeArray` "Continuer" :!type "Text")))
              (switch `/Game/SummerLearning/Blueprints/Dialogue/Enum_DialogueState` _state_3
                (:`NewEnumerator0`
                  (bind _state_4 (`self.AddDialogue` "Laura" "Mais sâches que si tu mets plus de rouge que de jaune, alors tu obtiendras un orange qui sera proche du rouge. " (`|MakeArray` "Continuer" :!type "Text")))
                  (switch `/Game/SummerLearning/Blueprints/Dialogue/Enum_DialogueState` _state_4
                    (:`NewEnumerator0`
                      (bind _state_5 (`self.AddDialogue` "Laura" "Et ça vaut pour toutes les couleurs ! Imagines le nombre de couleur que tu peux créer !" (`|MakeArray` "Continuer" :!type "Text")))
                      (switch `/Game/SummerLearning/Blueprints/Dialogue/Enum_DialogueState` _state_5
                        (:`NewEnumerator0`
                          (bind _state_6 (`self.AddDialogue` "Laura" "En tout cas, j'ai passé un super moment avec toi et j'espère que c'est pareil pour toi ! " (`|MakeArray` "Continuer" :!type "Text")))
                          (switch `/Game/SummerLearning/Blueprints/Dialogue/Enum_DialogueState` _state_6
                            (:`NewEnumerator0`
                              (bind _state_7 (`self.AddDialogue` "Laura" "A une prochaine fois ! " (`|MakeArray` "Continuer" :!type "Text")))
                              (switch `/Game/SummerLearning/Blueprints/Dialogue/Enum_DialogueState` _state_7
                                (:`NewEnumerator0`
                                  (`self.CloseConversation`))))))))))))))))))