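; BP_DeathZone_World2 is a kill volume for World 2 that sends the player back to their latest checkpoint when they overlap its box.
; It reads the four checkpoint flags on BP_BasePlayer in nested order, so a later checkpoint counts only if all earlier ones are set.
; It moves the player to a hardcoded world location for that progress level, or the start point, and zeroes the Shape's physics velocity.
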(event `self.Box.OnComponentBeginOverlap`
  (params (OverlappedComponent :type "PrimitiveComponent Object Reference") (OtherActor :type "Actor Object Reference") (OtherComp :type "PrimitiveComponent Object Reference") (OtherBodyIndex :type Integer) (bFromSweep :type Boolean) (SweepResult :type "HitResult Structure (by ref)"))
  (bind _asbp_base_player (cast `/Game/SummerLearning/Blueprints/Player/BP_BasePlayer` OtherActor))
  (if (`/Game/SummerLearning/Blueprints/Player/BP_BasePlayer.CheckpointOne` _asbp_base_player)
    (if (`/Game/SummerLearning/Blueprints/Player/BP_BasePlayer.CheckpointTwo` _asbp_base_player)
      (if (`/Game/SummerLearning/Blueprints/Player/BP_BasePlayer.CheckpointThree` _asbp_base_player)
        (if (`/Game/SummerLearning/Blueprints/Player/BP_BasePlayer.CheckpointFour` _asbp_base_player)
          (`self.K2_SetActorLocation` _asbp_base_player (13057.252233 -1048.116365 203.552552) false false)
          (bind _shape (`/Game/SummerLearning/Blueprints/Player/BP_BasePlayer.Shape` _asbp_base_player))
          (`PrimitiveComponent.SetPhysicsLinearVelocity` _shape (0.0 0.0 0.0) false "None")
          (else
            (`self.K2_SetActorLocation` _asbp_base_player (7327.537223 -3450.624892 -274.898288) false false)
            (`PrimitiveComponent.SetPhysicsLinearVelocity` _shape (0.0 0.0 0.0) false "None")))
        (else
          (`self.K2_SetActorLocation` _asbp_base_player (3971.100852 -2835.462571 -59.268912) false false)
          (`PrimitiveComponent.SetPhysicsLinearVelocity` _shape (0.0 0.0 0.0) false "None")))
      (else
        (`self.K2_SetActorLocation` _asbp_base_player (1910.972291 -1036.030425 237.635232) false false)
        (`PrimitiveComponent.SetPhysicsLinearVelocity` _shape (0.0 0.0 0.0) false "None")))
    (else
      (`self.K2_SetActorLocation` _asbp_base_player (291.206236 -1027.960274 165.321247) false false)
      (`PrimitiveComponent.SetPhysicsLinearVelocity` _shape (0.0 0.0 0.0) false "None"))))

(fn `UserConstructionScript`)