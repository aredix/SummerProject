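; Dialogue component for Laura's World 3 riddle, a French clown-nose puzzle solved by setting the player's color and shape.
; The first conversation chains AddDialogue lines, advances the tree index, then unlocks color and shape changing on BP_BasePlayer.
; Later conversations check the player's Color and Status, repeating the riddle if wrong.
; A correct answer destroys the riddle NPC, shows the World 4 transition NPC's mesh and enables passing through walls.
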(fn `Dialogue`
  (`parent.Dialogue`)
  (bind _asbp_base_player (cast `/Game/SummerLearning/Blueprints/Player/BP_BasePlayer` (`GameplayStatics.GetPlayerPawn` 0)))
  (switch `int` (`self.DialogueTreeIndex`)
    (:`0`
      (bind _state (`self.AddDialogue` "Laura" "Bien. Passons à une petite énigme." (`|MakeArray` "Continuer" :!type "Text")))
      (switch `/Game/SummerLearning/Blueprints/Dialogue/Enum_DialogueState` _state
        (:`NewEnumerator0`
          (bind _state_2 (`self.AddDialogue` "Laura" "Comme tu peux le voir, tu as à ta disposition 6 modificateurs." (`|MakeArray` "Continuer" :!type "Text")))
          (switch `/Game/SummerLearning/Blueprints/Dialogue/Enum_DialogueState` _state_2
            (:`NewEnumerator0`
              (bind _state_3 (`self.AddDialogue` "Laura" "Avec ces derniers, tu peux changer de couleurs et de formes." (`|MakeArray` "Continuer" :!type "Text")))
              (switch `/Game/SummerLearning/Blueprints/Dialogue/Enum_DialogueState` _state_3
                (:`NewEnumerator0`
                  (bind _state_4 (`self.AddDialogue` "Laura" "Voilà l'énigme. Je suis un clown et je porte un accessoire sur le nez. Quelle est sa forme ainsi que sa couleur ?" (`|MakeArray` "Continuer" :!type "Text")))
                  (switch `/Game/SummerLearning/Blueprints/Dialogue/Enum_DialogueState` _state_4
                    (:`NewEnumerator0`
                      (bind _state_5 (`self.AddDialogue` "Laura" "Reviens me voir avec la bonne réponse pour continuer !" (`|MakeArray` "Continuer" :!type "Text")))
                      (switch `/Game/SummerLearning/Blueprints/Dialogue/Enum_DialogueState` _state_5
                        (:`NewEnumerator0`
                          (bind _state_6 (`self.AddDialogue` "Laura" "Tu peux aussi revenir me voir pour réécouter l'énigme !" (`|MakeArray` "Continuer" :!type "Text")))
                          (switch `/Game/SummerLearning/Blueprints/Dialogue/Enum_DialogueState` _state_6
                            (:`NewEnumerator0`
                              (`self.SetDialogueTreeIndex` 1)
                              (`self.CloseConversation`)
                              (set `/Game/SummerLearning/Blueprints/Player/BP_BasePlayer.CanChangeColor` true _asbp_base_player)
                              (set `/Game/SummerLearning/Blueprints/Player/BP_BasePlayer.CanChangeShape` true _asbp_base_player))))))))))))))
    (:`1`
      (if (and (`|EnumEquality` (`/Game/SummerLearning/Blueprints/Player/BP_BasePlayer.Color` _asbp_base_player) "NewEnumerator3") (`|EnumEquality` (`/Game/SummerLearning/Blueprints/Player/BP_BasePlayer.Status` _asbp_base_player) "NewEnumerator3"))
        (bind _state_7 (`self.AddDialogue` "Laura" "Super ! Tu as trouvé la bonne réponse ! Rejoins moi de l'autre côté du mur !" (`|MakeArray` "Continuer" :!type "Text")))
        (switch `/Game/SummerLearning/Blueprints/Dialogue/Enum_DialogueState` _state_7
          (:`NewEnumerator0`
            (`self.SetDialogueTreeIndex` 1)
            (`self.CloseConversation`)
            (bind _returnvalue (`GameplayStatics.GetActorOfClass` "/Game/SummerLearning/Blueprints/Dialogue/World3/Enigme/BP_NPC_EnigmeWorld3.BP_NPC_EnigmeWorld3_C"))
            (`Actor.K2_DestroyActor` _returnvalue)
            (bind _returnvalue_2 (`GameplayStatics.GetActorOfClass` "/Game/SummerLearning/Blueprints/Dialogue/World3/ChangeToWorld4/BP_NPC_ChangeToWorld4.BP_NPC_ChangeToWorld4_C"))
            (`SceneComponent.SetVisibility` (`Character.Mesh` _returnvalue_2) true false)
            (set `/Game/SummerLearning/Blueprints/Player/BP_BasePlayer.CanPassThroughWalls` true _asbp_base_player)))
        (else
          (bind _state_8 (`self.AddDialogue` "Laura" "Oh ... Ce n'est pas la bonne réponse. Je vais te redire l'énigme." (`|MakeArray` "Continuer" :!type "Text")))
          (switch `/Game/SummerLearning/Blueprints/Dialogue/Enum_DialogueState` _state_8
            (:`NewEnumerator0`
              (bind _state_9 (`self.AddDialogue` "Laura" "Voilà l'énigme. Je suis un clown et je porte un accessoire sur le nez. Quelle est sa forme ainsi que sa couleur ?" (`|MakeArray` "Continuer" :!type "Text")))
              (switch `/Game/SummerLearning/Blueprints/Dialogue/Enum_DialogueState` _state_9
                (:`NewEnumerator0`
                  (`self.SetDialogueTreeIndex` 1)
                  (`self.CloseConversation`))))))))))