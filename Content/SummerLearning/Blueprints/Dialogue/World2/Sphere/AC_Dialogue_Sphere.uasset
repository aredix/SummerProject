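; Dialogue component for Laura's French-language sphere lesson in World 2, which asks the player to transform into a sphere.
; Branches on player Status: the first talk unlocks shape changing, and later talks repeat the requirement until it is met.
; The success branch explains spheres, destroys BP_NPC_Sphere, reveals BP_NPC_Enigme's mesh and lets the player pass through walls.
; Each branch increments its own dialogue counter on BP_BasePlayer.
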(fn `Dialogue`
  (`parent.Dialogue`)
  (bind _asbp_base_player (cast `/Game/SummerLearning/Blueprints/Player/BP_BasePlayer` (`GameplayStatics.GetPlayerPawn` 0)))
  (if (`|EnumInequality` (`/Game/SummerLearning/Blueprints/Player/BP_BasePlayer.Status` _asbp_base_player) "NewEnumerator3")
    (switch `int` (`self.DialogueTreeIndex`)
      (:`0`
        (`/Engine/EditorBlueprintResources/StandardMacros.IncrementInt` (`/Game/SummerLearning/Blueprints/Player/BP_BasePlayer.CompteurDialoguePrincipal` _asbp_base_player)
          (:`  `
            (bind _state (`self.AddDialogue` "Laura" "Eh bah, c'est sportif tout ça." (`|MakeArray` "Continuer" :!type "Text")))
            (switch `/Game/SummerLearning/Blueprints/Dialogue/Enum_DialogueState` _state
              (:`NewEnumerator0`
                (bind _state_2 (`self.AddDialogue` "Laura" "Bon, on est à nouveau face au même souci sauf que maintenant tu dois être une sphère." (`|MakeArray` "Continuer" :!type "Text")))
                (switch `/Game/SummerLearning/Blueprints/Dialogue/Enum_DialogueState` _state_2
                  (:`NewEnumerator0`
                    (bind _state_3 (`self.AddDialogue` "Laura" "Comme avant, tu peux changer ta forme en sphère. Transforme toi et reviens me voir." (`|MakeArray` "Continuer" :!type "Text")))
                    (switch `/Game/SummerLearning/Blueprints/Dialogue/Enum_DialogueState` _state_3
                      (:`NewEnumerator0`
                        (`self.SetDialogueTreeIndex` 1)
                        (`self.CloseConversation`)
                        (set `/Game/SummerLearning/Blueprints/Player/BP_BasePlayer.CanChangeShape` true _asbp_base_player))))))))))
      (:`1`
        (`/Engine/EditorBlueprintResources/StandardMacros.IncrementInt` (`/Game/SummerLearning/Blueprints/Player/BP_BasePlayer.CompteurDialogueErreur` _asbp_base_player)
          (:`  `
            (bind _state_4 (`self.AddDialogue` "Laura" "Tu dois être une sphère pour pouvoir continuer." (`|MakeArray` "Continuer" :!type "Text")))
            (switch `/Game/SummerLearning/Blueprints/Dialogue/Enum_DialogueState` _state_4
              (:`NewEnumerator0`
                (`self.SetDialogueTreeIndex` 1)
                (`self.CloseConversation`)))))))
    (else
      (switch `int` (`self.DialogueTreeIndex2`)
        (:`0`
          (`/Engine/EditorBlueprintResources/StandardMacros.IncrementInt` (`/Game/SummerLearning/Blueprints/Player/BP_BasePlayer.CompteurDialogueSuite` _asbp_base_player)
            (:`  `
              (bind _state_5 (`self.AddDialogue` "Laura" "Super ! Une sphère est une face arrondie, comme une balle (ou la Terre)" (`|MakeArray` "Continuer" :!type "Text")))
              (switch `/Game/SummerLearning/Blueprints/Dialogue/Enum_DialogueState` _state_5
                (:`NewEnumerator0`
                  (bind _state_6 (`self.AddDialogue` "Laura" "Rejoins-moi de l'autre côté du mur maintenant." (`|MakeArray` "Continuer" :!type "Text")))
                  (switch `/Game/SummerLearning/Blueprints/Dialogue/Enum_DialogueState` _state_6
                    (:`NewEnumerator0`
                      (set `self.DialogueTreeIndex2` 1)
                      (`self.ClearDialogueProgress`)
                      (`self.CloseConversation`)
                      (bind _returnvalue (`GameplayStatics.GetActorOfClass` "/Game/SummerLearning/Blueprints/Dialogue/World2/Sphere/BP_NPC_Sphere.BP_NPC_Sphere_C"))
                      (`Actor.K2_DestroyActor` _returnvalue)
                      (bind _returnvalue_2 (`GameplayStatics.GetActorOfClass` "/Game/SummerLearning/Blueprints/Dialogue/World2/Enigme/BP_NPC_Enigme.BP_NPC_Enigme_C"))
                      (`SceneComponent.SetVisibility` (`Character.Mesh` _returnvalue_2) true false)
                      (set `/Game/SummerLearning/Blueprints/Player/BP_BasePlayer.CanPassThroughWalls` true _asbp_base_player))))))))))))