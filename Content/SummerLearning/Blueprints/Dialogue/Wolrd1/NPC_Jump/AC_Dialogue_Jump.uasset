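; Dialogue component for the World 1 jump tutorial, where Laura explains in French that the bridge is broken and teaches jumping with the space bar.
; It overrides Dialogue with a linear chain of single-option AddDialogue lines.
; The last line advances the tree index, closes the conversation, enables CanJump on BP_BasePlayer, destroys BP_NPC_Jump and reveals the mesh of BP_NPC_ChangeToWolrd2.
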(fn `Dialogue`
  (`parent.Dialogue`)
  (switch `int` (`self.DialogueTreeIndex`)
    (:`0`
      (bind _state (`self.AddDialogue` "Laura" "Ah te voilà !" (`|MakeArray` "Continuer" :!type "Text")))
      (switch `/Game/SummerLearning/Blueprints/Dialogue/Enum_DialogueState` _state
        (:`NewEnumerator0`
          (bind _state_2 (`self.AddDialogue` "Laura" "On a un petit souci. Le pont qui nous permettait de continuer est cassé." (`|MakeArray` "Continuer" :!type "Text")))
          (switch `/Game/SummerLearning/Blueprints/Dialogue/Enum_DialogueState` _state_2
            (:`NewEnumerator0`
              (bind _state_3 (`self.AddDialogue` "Laura" "On va devoir sauter par dessus. " (`|MakeArray` "Continuer" :!type "Text")))
              (switch `/Game/SummerLearning/Blueprints/Dialogue/Enum_DialogueState` _state_3
                (:`NewEnumerator0`
                  (bind _state_4 (`self.AddDialogue` "Laura" "Pour se faire, utilise la barre espace pour me rejoindre de l'autre côté." (`|MakeArray` "Continuer" :!type "Text")))
                  (switch `/Game/SummerLearning/Blueprints/Dialogue/Enum_DialogueState` _state_4
                    (:`NewEnumerator0`
                      (bind _state_5 (`self.AddDialogue` "Laura" "Je t'attends de l'autre côté !" (`|MakeArray` "Continuer" :!type "Text")))
                      (switch `/Game/SummerLearning/Blueprints/Dialogue/Enum_DialogueState` _state_5
                        (:`NewEnumerator0`
                          (`self.SetDialogueTreeIndex` 1)
                          (`self.CloseConversation`)
                          (bind _asbp_base_player (cast `/Game/SummerLearning/Blueprints/Player/BP_BasePlayer` (`GameplayStatics.GetPlayerPawn` 0)))
                          (set `/Game/SummerLearning/Blueprints/Player/BP_BasePlayer.CanJump` true _asbp_base_player)
                          (bind _returnvalue (`GameplayStatics.GetActorOfClass` "/Game/SummerLearning/Blueprints/Dialogue/Wolrd1/NPC_Jump/BP_NPC_Jump.BP_NPC_Jump_C"))
                          (`Actor.K2_DestroyActor` _returnvalue)
                          (bind _returnvalue_2 (`GameplayStatics.GetActorOfClass` "/Game/SummerLearning/Blueprints/Dialogue/Wolrd1/NPC_ChangeToWorld2/BP_NPC_ChangeToWolrd2.BP_NPC_ChangeToWolrd2_C"))
                          (`SceneComponent.SetVisibility` (`Character.Mesh` _returnvalue_2) true false))))))))))))))