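; Dialogue component for the Violet NPC in World 4, where Laura teaches color mixing in French.
; An overridden Dialogue graph branches on DialogueTreeIndex: the intro unlocks the player's mixing, color change and reset, then advances to a color check.
; A correct color enables passing through walls, destroys this NPC and reveals the Orange NPC's mesh, while a wrong one repeats the check.
; Each branch increments its own dialogue counter on the player.
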(fn `Dialogue`
  (`parent.Dialogue`)
  (bind _asbp_base_player (cast `/Game/SummerLearning/Blueprints/Player/BP_BasePlayer` (`GameplayStatics.GetPlayerPawn` 0)))
  (switch `int` (`self.DialogueTreeIndex`)
    (:`0`
      (`/Engine/EditorBlueprintResources/StandardMacros.IncrementInt` (`/Game/SummerLearning/Blueprints/Player/BP_BasePlayer.CompteurDialoguePrincipal` _asbp_base_player)
        (:`  `
          (bind _state (`self.AddDialogue` "Laura" "Nous voilà à présent au dernier monde, le monde des mélanges de couleurs." (`|MakeArray` "Continuer" :!type "Text")))
          (switch `/Game/SummerLearning/Blueprints/Dialogue/Enum_DialogueState` _state
            (:`NewEnumerator0`
              (bind _state_2 (`self.AddDialogue` "Laura" "Dans ce monde, en combinant les couleurs entre elles, tu peux créer une toute nouvelle couleur ! " (`|MakeArray` "Continuer" :!type "Text")))
              (switch `/Game/SummerLearning/Blueprints/Dialogue/Enum_DialogueState` _state_2
                (:`NewEnumerator0`
                  (bind _state_3 (`self.AddDialogue` "Laura" "C'est un peu comme de la magie tu ne trouves pas ? " (`|MakeArray` "Continuer" :!type "Text")))
                  (switch `/Game/SummerLearning/Blueprints/Dialogue/Enum_DialogueState` _state_3
                    (:`NewEnumerator0`
                      (bind _state_4 (`self.AddDialogue` "Laura" "Mais rassure-toi, nous n'allons découvrir que les mélanges issus des couleurs que nous avons vu précédemment." (`|MakeArray` "Continuer" :!type "Text")))
                      (switch `/Game/SummerLearning/Blueprints/Dialogue/Enum_DialogueState` _state_4
                        (:`NewEnumerator0`
                          (bind _state_5 (`self.AddDialogue` "Laura" "Comme tu peux le voir, la couleur du mur dans lequel tu dois passer est violette." (`|MakeArray` "Continuer" :!type "Text")))
                          (switch `/Game/SummerLearning/Blueprints/Dialogue/Enum_DialogueState` _state_5
                            (:`NewEnumerator0`
                              (bind _state_6 (`self.AddDialogue` "Laura" "Je t'ai accroché juste à côté un petit tableau qui t'explique comment fonctionne les mélanges." (`|MakeArray` "Continuer" :!type "Text")))
                              (switch `/Game/SummerLearning/Blueprints/Dialogue/Enum_DialogueState` _state_6
                                (:`NewEnumerator0`
                                  (bind _state_7 (`self.AddDialogue` "Laura" "Si tu te trompes dans un mélange, tu peux recommencer en appuyant sur ta touche R." (`|MakeArray` "Continuer" :!type "Text")))
                                  (switch `/Game/SummerLearning/Blueprints/Dialogue/Enum_DialogueState` _state_7
                                    (:`NewEnumerator0`
                                      (bind _state_8 (`self.AddDialogue` "Laura" "Reproduis la couleur violette et reviens me voir !" (`|MakeArray` "Continuer" :!type "Text")))
                                      (switch `/Game/SummerLearning/Blueprints/Dialogue/Enum_DialogueState` _state_8
                                        (:`NewEnumerator0`
                                          (set `/Game/SummerLearning/Blueprints/Player/BP_BasePlayer.CanMixColor` true _asbp_base_player)
                                          (set `/Game/SummerLearning/Blueprints/Player/BP_BasePlayer.CanChangeColor` true _asbp_base_player)
                                          (`self.SetDialogueTreeIndex` 1)
                                          (`self.SetDialogueTreeIndex` 1)
                                          (`self.CloseConversation`)
                                          (set `/Game/SummerLearning/Blueprints/Player/BP_BasePlayer.CanReset` true _asbp_base_player))))))))))))))))))))
    (:`1`
      (if (`|EnumEquality` (`/Game/SummerLearning/Blueprints/Player/BP_BasePlayer.Color` _asbp_base_player) "NewEnumerator0")
        (`/Engine/EditorBlueprintResources/StandardMacros.IncrementInt` (`/Game/SummerLearning/Blueprints/Player/BP_BasePlayer.CompteurDialogueSuite` _asbp_base_player)
          (:`  `
            (bind _state_9 (`self.AddDialogue` "Laura" "Super ! Tu as réussi à faire le bon mélange de couleurs." (`|MakeArray` "Continuer" :!type "Text")))
            (switch `/Game/SummerLearning/Blueprints/Dialogue/Enum_DialogueState` _state_9
              (:`NewEnumerator0`
                (bind _state_10 (`self.AddDialogue` "Laura" "Tu peux à présent me rejoindre de l'autre côté pour continuer à découvrir de nouvelles couleurs." (`|MakeArray` "Continuer" :!type "Text")))
                (switch `/Game/SummerLearning/Blueprints/Dialogue/Enum_DialogueState` _state_10
                  (:`NewEnumerator0`
                    (set `/Game/SummerLearning/Blueprints/Player/BP_BasePlayer.CanPassThroughWalls` true _asbp_base_player)
                    (`self.CloseConversation`)
                    (bind _returnvalue (`GameplayStatics.GetActorOfClass` "/Game/SummerLearning/Blueprints/Dialogue/World4/NPC_Violet/BP_NPC_Violet.BP_NPC_Violet_C"))
                    (`Actor.K2_DestroyActor` _returnvalue)
                    (bind _returnvalue_2 (`GameplayStatics.GetActorOfClass` "/Game/SummerLearning/Blueprints/Dialogue/World4/NPC_Orange/BP_NPC_Orange.BP_NPC_Orange_C"))
                    (`SceneComponent.SetVisibility` (`Character.Mesh` _returnvalue_2) true false)))))))
        (else
          (`/Engine/EditorBlueprintResources/StandardMacros.IncrementInt` (`/Game/SummerLearning/Blueprints/Player/BP_BasePlayer.CompteurDialogueErreur` _asbp_base_player)
            (:`  `
              (bind _state_11 (`self.AddDialogue` "Laura" "Malhreusement tu n'as pas la bonne couleur. Consulte le tableau et effectue le bon mélange. " (`|MakeArray` "Continuer" :!type "Text")))
              (switch `/Game/SummerLearning/Blueprints/Dialogue/Enum_DialogueState` _state_11
                (:`NewEnumerator0`
                  (bind _state_12 (`self.AddDialogue` "Laura" "N'oublis pas que si tu fais une erreur, tu as besoin de réinitialiser ta couleur avec la touche R." (`|MakeArray` "Continuer" :!type "Text")))
                  (switch `/Game/SummerLearning/Blueprints/Dialogue/Enum_DialogueState` _state_12
                    (:`NewEnumerator0`
                      (`self.CloseConversation`)
                      (`self.SetDialogueTreeIndex` 1))))))))))))