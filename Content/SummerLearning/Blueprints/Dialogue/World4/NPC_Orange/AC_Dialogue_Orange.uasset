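; Dialogue component for Laura, the orange NPC in World 4, who gives the player a French-language lesson on mixing orange.
; It overrides the parent Dialogue function and branches on DialogueTreeIndex: the intro enables colour change and mixing, then later talks check the player's colour.
; Success enables passing through walls, destroys BP_NPC_Orange and reveals BP_NPC_Vert's mesh; failure gives a reset hint and allows retrying.
; Each branch also increments a dialogue counter on the player.
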(fn `Dialogue`
  (`parent.Dialogue`)
  (bind _asbp_base_player (cast `/Game/SummerLearning/Blueprints/Player/BP_BasePlayer` (`GameplayStatics.GetPlayerPawn` 0)))
  (switch `int` (`self.DialogueTreeIndex`)
    (:`0`
      (`/Engine/EditorBlueprintResources/StandardMacros.IncrementInt` (`/Game/SummerLearning/Blueprints/Player/BP_BasePlayer.CompteurDialoguePrincipal` _asbp_base_player)
        (:`  `
          (bind _state (`self.AddDialogue` "Laura" "Bien, maintenant observe le tableau et essaye de reproduire la couleur orange." (`|MakeArray` "Continuer" :!type "Text")))
          (switch `/Game/SummerLearning/Blueprints/Dialogue/Enum_DialogueState` _state
            (:`NewEnumerator0`
              (bind _state_2 (`self.AddDialogue` "Laura" "Tu peux retrouver la couleur orange sur certains fruits commes les clémantines ou encore, les abricots." (`|MakeArray` "Continuer" :!type "Text")))
              (switch `/Game/SummerLearning/Blueprints/Dialogue/Enum_DialogueState` _state_2
                (:`NewEnumerator0`
                  (bind _state_3 (`self.AddDialogue` "Laura" "Reviens me voir quand c'est fait." (`|MakeArray` "Continuer" :!type "Text")))
                  (switch `/Game/SummerLearning/Blueprints/Dialogue/Enum_DialogueState` _state_3
                    (:`NewEnumerator0`
                      (`self.CloseConversation`)
                      (set `/Game/SummerLearning/Blueprints/Player/BP_BasePlayer.CanChangeColor` true _asbp_base_player)
                      (set `/Game/SummerLearning/Blueprints/Player/BP_BasePlayer.CanMixColor` true _asbp_base_player)
                      (`self.SetDialogueTreeIndex` 1))))))))))
    (:`1`
      (if (`|EnumEquality` (`/Game/SummerLearning/Blueprints/Player/BP_BasePlayer.Color` _asbp_base_player) "NewEnumerator2")
        (`/Engine/EditorBlueprintResources/StandardMacros.IncrementInt` (`/Game/SummerLearning/Blueprints/Player/BP_BasePlayer.CompteurDialogueSuite` _asbp_base_player)
          (:`  `
            (bind _state_4 (`self.AddDialogue` "Laura" "Super ! Je vois que tu apprends vite ! Rejoins moi de l'autre côté pour continuer." (`|MakeArray` "Continuer" :!type "Text")))
            (switch `/Game/SummerLearning/Blueprints/Dialogue/Enum_DialogueState` _state_4
              (:`NewEnumerator0`
                (set `/Game/SummerLearning/Blueprints/Player/BP_BasePlayer.CanPassThroughWalls` true _asbp_base_player)
                (`self.CloseConversation`)
                (bind _returnvalue (`GameplayStatics.GetActorOfClass` "/Game/SummerLearning/Blueprints/Dialogue/World4/NPC_Orange/BP_NPC_Orange.BP_NPC_Orange_C"))
                (`Actor.K2_DestroyActor` _returnvalue)
                (bind _returnvalue_2 (`GameplayStatics.GetActorOfClass` "/Game/SummerLearning/Blueprints/Dialogue/World4/NPC_Vert/BP_NPC_Vert.BP_NPC_Vert_C"))
                (`SceneComponent.SetVisibility` (`Character.Mesh` _returnvalue_2) true false)))))
        (else
          (`/Engine/EditorBlueprintResources/StandardMacros.IncrementInt` (`/Game/SummerLearning/Blueprints/Player/BP_BasePlayer.CompteurDialogueErreur` _asbp_base_player)
            (:`  `
              (bind _state_5 (`self.AddDialogue` "Laura" "Malhreusement tu n'as pas la bonne couleur. Consulte le tableau et effectue le bon mélange. " (`|MakeArray` "Continuer" :!type "Text")))
              (switch `/Game/SummerLearning/Blueprints/Dialogue/Enum_DialogueState` _state_5
                (:`NewEnumerator0`
                  (bind _state_6 (`self.AddDialogue` "Laura" "N'oublis pas que si tu fais une erreur, tu as besoin de réinitialiser ta couleur avec la touche R." (`|MakeArray` "Continuer" :!type "Text")))
                  (switch `/Game/SummerLearning/Blueprints/Dialogue/Enum_DialogueState` _state_6
                    (:`NewEnumerator0`
                      (`self.CloseConversation`)
                      (`self.SetDialogueTreeIndex` 1))))))))))))