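; Death zone volume for World 3 that sends the player back to their latest checkpoint on contact.
; When a BP_BasePlayer overlaps its Box, nested checks of the player's four checkpoint flags, in order, pick one of five hardcoded world locations, including a default when the first is unset.
; The player is moved there and the linear velocity of its physics Shape is zeroed.
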(event `self.Box.OnComponentBeginOverlap`
  (params (OverlappedComponent :type "PrimitiveComponent Object Reference") (OtherActor :type "Actor Object Reference") (OtherComp :type "PrimitiveComponent Object Reference") (OtherBodyIndex :type Integer) (bFromSweep :type Boolean) (SweepResult :type "HitResult Structure (by ref)"))
  (bind _asbp_base_player (cast `/Game/SummerLearning/Blueprints/Player/BP_BasePlayer` OtherActor))
  (if (`/Game/SummerLearning/Blueprints/Player/BP_BasePlayer.CheckpointOne` _asbp_base_player)
    (if (`/Game/SummerLearning/Blueprints/Player/BP_BasePlayer.CheckpointTwo` _asbp_base_player)
      (if (`/Game/SummerLearning/Blueprints/Player/BP_BasePlayer.CheckpointThree` _asbp_base_player)
        (if (`/Game/SummerLearning/Blueprints/Player/BP_BasePlayer.CheckpointFour` _asbp_base_player)
          (`self.K2_SetActorLocation` _asbp_base_player (-3550.503655 -3672.578302 1068.221997) false false)
          (bind _shape (`/Game/SummerLearning/Blueprints/Player/BP_BasePlayer.Shape` _asbp_base_player))
          (`PrimitiveComponent.SetPhysicsLinearVelocity` _shape (0.0 0.0 0.0) false "None")
          (else
            (`self.K2_SetActorLocation` _asbp_base_player (64.257925 -4276.671365 746.995885) false false)
            (`PrimitiveComponent.SetPhysicsLinearVelocity` _shape (0.0 0.0 0.0) false "None")))
        (else
          (`self.K2_SetActorLocation` _asbp_base_player (2424.601377 -4850.145366 577.075647) false false)
          (`PrimitiveComponent.SetPhysicsLinearVelocity` _shape (0.0 0.0 0.0) false "None")))
      (else
        (`self.K2_SetActorLocation` _asbp_base_player (1910.972291 -1036.030425 237.635232) false false)
        (`PrimitiveComponent.SetPhysicsLinearVelocity` _shape (0.0 0.0 0.0) false "None")))
    (else
      (`self.K2_SetActorLocation` _asbp_base_player (140.723786 -1228.311672 179.791144) false false)
      (`PrimitiveComponent.SetPhysicsLinearVelocity` _shape (0.0 0.0 0.0) false "None"))))

(fn `UserConstructionScript`)