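; Dialogue component for the World 1 NPC that sends the player to World 2 in the SummerLearning game.
; It extends a parent dialogue, switches on the tree index and increments the player's main dialogue counter.
; Laura offers a single option, and once the line passes through, the conversation closes and the shapes level LVL_2_Formes opens.
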(fn `Dialogue`
  (`parent.Dialogue`)
  (bind _asbp_base_player (cast `/Game/SummerLearning/Blueprints/Player/BP_BasePlayer` (`GameplayStatics.GetPlayerPawn` 0)))
  (switch `int` (`self.DialogueTreeIndex`)
    (:`0`
      (`/Engine/EditorBlueprintResources/StandardMacros.IncrementInt` (`/Game/SummerLearning/Blueprints/Player/BP_BasePlayer.CompteurDialoguePrincipal` _asbp_base_player)
        (:`  `
          (bind _state (`self.AddDialogue` "Laura" "Super ! Allez, allons au monde suivant !" (`|MakeArray` "Passer au monde 2" :!type "Text")))
          (switch `/Game/SummerLearning/Blueprints/Dialogue/Enum_DialogueState` _state
            (:`NewEnumerator0`
              (`self.CloseConversation`)
              (`GameplayStatics.OpenLevel` "LVL_2_Formes"))))))))