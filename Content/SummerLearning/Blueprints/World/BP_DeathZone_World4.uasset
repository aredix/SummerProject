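; Death zone for World 4 that sends the player back to their latest checkpoint when they overlap its Box trigger.
; On overlap it casts to BP_BasePlayer and checks the four checkpoint flags in nested order, so the first unset flag decides the respawn point.
; Respawn positions are hardcoded world locations, one per checkpoint plus a start point.
; Each respawn moves the player without sweep and zeroes the Shape's physics linear velocity.
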(event `self.Box.OnComponentBeginOverlap`
  (params (OverlappedComponent :type "PrimitiveComponent Object Reference") (OtherActor :type "Actor Object Reference") (OtherComp :type "PrimitiveComponent Object Reference") (OtherBodyIndex :type Integer) (bFromSweep :type Boolean) (SweepResult :type "HitResult Structure (by ref)"))
  (bind _asbp_base_player (cast `/Game/SummerLearning/Blueprints/Player/BP_BasePlayer` OtherActor))
  (if (`/Game/SummerLearning/Blueprints/Player/BP_BasePlayer.CheckpointOne` _asbp_base_player)
    (if (`/Game/SummerLearning/Blueprints/Player/BP_BasePlayer.CheckpointTwo` _asbp_base_player)
      (if (`/Game/SummerLearning/Blueprints/Player/BP_BasePlayer.CheckpointThree` _asbp_base_player)
        (if (`/Game/SummerLearning/Blueprints/Player/BP_BasePlayer.CheckpointFour` _asbp_base_player)
          (`self.K2_SetActorLocation` _asbp_base_player (12728.81339 -1414.117086 1044.585084) false false)
          (bind _shape (`/Game/SummerLearning/Blueprints/Player/BP_BasePlayer.Shape` _asbp_base_player))
          (`PrimitiveComponent.SetPhysicsLinearVelocity` _shape (0.0 0.0 0.0) false "None")
          (else
            (`self.K2_SetActorLocation` _asbp_base_player (8652.035821 -1414.117086 827.771143) false false)
            (`PrimitiveComponent.SetPhysicsLinearVelocity` _shape (0.0 0.0 0.0) false "None")))
        (else
          (`self.K2_SetActorLocation` _asbp_base_player (5412.055217 -1414.117065 562.700678) false false)
          (`PrimitiveComponent.SetPhysicsLinearVelocity` _shape (0.0 0.0 0.0) false "None")))
      (else
        (`self.K2_SetActorLocation` _asbp_base_player (1522.365753 -1414.117064 240.436796) false false)
        (`PrimitiveComponent.SetPhysicsLinearVelocity` _shape (0.0 0.0 0.0) false "None")))
    (else
      (`self.K2_SetActorLocation` _asbp_base_player (75.88409 -1464.475634 165.32126) false false)
      (`PrimitiveComponent.SetPhysicsLinearVelocity` _shape (0.0 0.0 0.0) false "None"))))

(fn `UserConstructionScript`)