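; Dialogue component for Laura, the World 4 riddle NPC, who asks the player to take a brick's shape and color from memory.
; The first conversation explains the riddle, enables color change, mixing and shape change, then advances DialogueTreeIndex.
; Later talks check only the player's color, repeating hints if wrong.
; Success grants wall pass-through, destroys BP_NPC_EnigmeWorld4 and reveals BP_NPC_Fin's mesh.
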(fn `Dialogue`
  (`parent.Dialogue`)
  (bind _asbp_base_player (cast `/Game/SummerLearning/Blueprints/Player/BP_BasePlayer` (`GameplayStatics.GetPlayerPawn` 0)))
  (switch `int` (`self.DialogueTreeIndex`)
    (:`0`
      (bind _state (`self.AddDialogue` "Laura" "Super, afin de voir si tu astout retenu, je te laisse répondre à cette énigme." (`|MakeArray` "Continuer" :!type "Text")))
      (switch `/Game/SummerLearning/Blueprints/Dialogue/Enum_DialogueState` _state
        (:`NewEnumerator0`
          (bind _state_2 (`self.AddDialogue` "Laura" "Pour cette énigme, tu n'auras pas le tableau à ta disposition. Tu devras donc faire appel à ta mémorie." (`|MakeArray` "Continuer" :!type "Text")))
          (switch `/Game/SummerLearning/Blueprints/Dialogue/Enum_DialogueState` _state_2
            (:`NewEnumerator0`
              (bind _state_3 (`self.AddDialogue` "Laura" "N'oublis pas qu'en cas d'erreur, tu peux réinitialiser ta couleur avec la touche R." (`|MakeArray` "Continuer" :!type "Text")))
              (switch `/Game/SummerLearning/Blueprints/Dialogue/Enum_DialogueState` _state_3
                (:`NewEnumerator0`
                  (bind _state_4 (`self.AddDialogue` "Laura" "J'aimerai que tu prennes la forme et la couleur d'une brique." (`|MakeArray` "Continuer" :!type "Text")))
                  (switch `/Game/SummerLearning/Blueprints/Dialogue/Enum_DialogueState` _state_4
                    (:`NewEnumerator0`
                      (`self.CloseConversation`)
                      (`self.SetDialogueTreeIndex` 1)
                      (set `/Game/SummerLearning/Blueprints/Player/BP_BasePlayer.CanChangeColor` true _asbp_base_player)
                      (set `/Game/SummerLearning/Blueprints/Player/BP_BasePlayer.CanMixColor` true _asbp_base_player)
                      (set `/Game/SummerLearning/Blueprints/Player/BP_BasePlayer.CanChangeShape` true _asbp_base_player))))))))))
    (:`1`
      (if (`|EnumEquality` (`/Game/SummerLearning/Blueprints/Player/BP_BasePlayer.Color` _asbp_base_player) "NewEnumerator2")
        (bind _state_5 (`self.AddDialogue` "Laura" "Super ! Tu as réussi à résoudre la dernière énigme !" (`|MakeArray` "Continuer" :!type "Text")))
        (switch `/Game/SummerLearning/Blueprints/Dialogue/Enum_DialogueState` _state_5
          (:`NewEnumerator0`
            (bind _state_6 (`self.AddDialogue` "Laura" "Je t'invite à me rejoindre de l'autre côté." (`|MakeArray` "Continuer" :!type "Text")))
            (switch `/Game/SummerLearning/Blueprints/Dialogue/Enum_DialogueState` _state_6
              (:`NewEnumerator0`
                (set `/Game/SummerLearning/Blueprints/Player/BP_BasePlayer.CanPassThroughWalls` true _asbp_base_player)
                (`self.CloseConversation`)
                (bind _returnvalue (`GameplayStatics.GetActorOfClass` "/Game/SummerLearning/Blueprints/Dialogue/World4/NPC_Enigme/BP_NPC_EnigmeWorld4.BP_NPC_EnigmeWorld4_C"))
                (`Actor.K2_DestroyActor` _returnvalue)
                (bind _returnvalue_2 (`GameplayStatics.GetActorOfClass` "/Game/SummerLearning/Blueprints/Dialogue/World4/NPC_Fin/BP_NPC_Fin.BP_NPC_Fin_C"))
                (`SceneComponent.SetVisibility` (`Character.Mesh` _returnvalue_2) true false)))))
        (else
          (bind _state_7 (`self.AddDialogue` "Laura" "Malhreusement tu n'as pas la bonne couleur. Consulte le tableau et effectue le bon mélange. " (`|MakeArray` "Continuer" :!type "Text")))
          (switch `/Game/SummerLearning/Blueprints/Dialogue/Enum_DialogueState` _state_7
            (:`NewEnumerator0`
              (bind _state_8 (`self.AddDialogue` "Laura" "Il faut que tu prennes la forme et la couleur d'une brique." (`|MakeArray` "Continuer" :!type "Text")))
              (switch `/Game/SummerLearning/Blueprints/Dialogue/Enum_DialogueState` _state_8
                (:`NewEnumerator0`
                  (bind _state_9 (`self.AddDialogue` "Laura" "N'oublis pas que si tu fais une erreur, tu as besoin de réinitialiser ta couleur avec la touche R." (`|MakeArray` "Continuer" :!type "Text")))
                  (switch `/Game/SummerLearning/Blueprints/Dialogue/Enum_DialogueState` _state_9
                    (:`NewEnumerator0`
                      (`self.CloseConversation`)
                      (`self.SetDialogueTreeIndex` 1))))))))))))