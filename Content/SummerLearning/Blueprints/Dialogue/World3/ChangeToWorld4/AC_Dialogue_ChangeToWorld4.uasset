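; Dialogue component for the World 3 exit, where Laura congratulates the player in French and sends them on to World 4.
; The overridden Dialogue function calls its parent, then adds a single line with one "Continuer" option.
; On the Pass Through state it closes the conversation, sets the BP_BasePlayer shape to the cube mesh and its status to the enum's NewEnumerator0, then opens LVL_4_Melanges.
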(fn `Dialogue`
  (`parent.Dialogue`)
  (bind _state (`self.AddDialogue` "Laura" "Bien joué ! Tu as compris ! Maintenant, allons au monde suivant." (`|MakeArray` "Continuer" :!type "Text")))
  (switch `/Game/SummerLearning/Blueprints/Dialogue/Enum_DialogueState` _state
    (:`NewEnumerator0`
      (`self.CloseConversation`)
      (bind _asbp_base_player (cast `/Game/SummerLearning/Blueprints/Player/BP_BasePlayer` (`GameplayStatics.GetPlayerPawn` 0)))
      (`StaticMeshComponent.SetStaticMesh` (`/Game/SummerLearning/Blueprints/Player/BP_BasePlayer.Shape` _asbp_base_player) "/Game/SummerLearning/Blueprints/Player/StaticMeshes/SM_PlayerCube.SM_PlayerCube")
      (set `/Game/SummerLearning/Blueprints/Player/BP_BasePlayer.Status` "NewEnumerator0" _asbp_base_player)
      (`GameplayStatics.OpenLevel` "LVL_4_Melanges"))))