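; BP_ColorChangeToBlue is a world trigger that recolors the player blue when its ChangeColor component is overlapped.
; It acts only on a BP_BasePlayer with CanChangeColor, setting both the Shape material and the Color state.
; Yellow or red players with NeedReset set instead mix to green or violet if CanMixColor allows, otherwise keep their color.
; All other cases become blue.
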(event `self.ChangeColor.OnComponentBeginOverlap`
  (params (OverlappedComponent :type "PrimitiveComponent Object Reference") (OtherActor :type "Actor Object Reference") (OtherComp :type "PrimitiveComponent Object Reference") (OtherBodyIndex :type Integer) (bFromSweep :type Boolean) (SweepResult :type "HitResult Structure (by ref)"))
  (bind _asbp_base_player (cast `/Game/SummerLearning/Blueprints/Player/BP_BasePlayer` OtherActor))
  (if (`/Game/SummerLearning/Blueprints/Player/BP_BasePlayer.CanChangeColor` _asbp_base_player)
    (switch `/Game/SummerLearning/Blueprints/Player/PlayerColorStatus` (`/Game/SummerLearning/Blueprints/Player/BP_BasePlayer.Color` _asbp_base_player)
      (:`NewEnumerator6`
        (bind _shape (`/Game/SummerLearning/Blueprints/Player/BP_BasePlayer.Shape` _asbp_base_player))
        (`PrimitiveComponent.SetMaterial` _shape 0 "/Game/SummerLearning/Materials/M_Blue.M_Blue" :!label _label)
        (set `/Game/SummerLearning/Blueprints/Player/BP_BasePlayer.Color` "NewEnumerator5" _asbp_base_player))
      (:`NewEnumerator1`
        (bind _needreset (`/Game/SummerLearning/Blueprints/Player/BP_BasePlayer.NeedReset` _asbp_base_player))
        (if _needreset
          (bind _canmixcolor (`/Game/SummerLearning/Blueprints/Player/BP_BasePlayer.CanMixColor` _asbp_base_player))
          (if _canmixcolor
            (`PrimitiveComponent.SetMaterial` _shape 0 "/Game/SummerLearning/Materials/M_Green.M_Green")
            (set `/Game/SummerLearning/Blueprints/Player/BP_BasePlayer.Color` "NewEnumerator4" _asbp_base_player))
          (else
            (goto _label))))
      (:`NewEnumerator3`
        (if _needreset
          (if _canmixcolor
            (`PrimitiveComponent.SetMaterial` _shape 0 "/Game/SummerLearning/Materials/M_Violet.M_Violet")
            (set `/Game/SummerLearning/Blueprints/Player/BP_BasePlayer.Color` "NewEnumerator0" _asbp_base_player))
          (else
            (goto _label))))
      (:`NewEnumerator5`
        (goto _label)))))

(fn `UserConstructionScript`)