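; Dialogue component for Laura in World 2's rectangle lesson, guiding the player to turn from a cube into a rectangle to pass a wall.
; It overrides Dialogue and picks one of two branches from the player's Status, before or after the shape change.
; Each branch chains French AddDialogue lines, then uses its own tree index to repeat a short reminder on later talks.
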(fn `Dialogue`
  (`parent.Dialogue`)
  (bind _asbp_base_player (cast `/Game/SummerLearning/Blueprints/Player/BP_BasePlayer` (`GameplayStatics.GetPlayerPawn` 0)))
  (if (`|EnumInequality` (`/Game/SummerLearning/Blueprints/Player/BP_BasePlayer.Status` _asbp_base_player) "NewEnumerator1")
    (switch `int` (`self.DialogueTreeIndex`)
      (:`0`
        (bind _state (`self.AddDialogue` "Laura" "Bien ! Bon maintenant, on est face à un petit soucis..." (`|MakeArray` "Continuer" :!type "Text")))
        (switch `/Game/SummerLearning/Blueprints/Dialogue/Enum_DialogueState` _state
          (:`NewEnumerator0`
            (bind _state_2 (`self.AddDialogue` "Laura" "Tu es un cube mais la forme dans le mur est un rectangle ..." (`|MakeArray` "Continuer" :!type "Text")))
            (switch `/Game/SummerLearning/Blueprints/Dialogue/Enum_DialogueState` _state_2
              (:`NewEnumerator0`
                (bind _state_3 (`self.AddDialogue` "Laura" "Oh ! Regardes ! Derrière toi tu peux changer ta forme en rectangle !" (`|MakeArray` "Regarder derrière" :!type "Text")))
                (switch `/Game/SummerLearning/Blueprints/Dialogue/Enum_DialogueState` _state_3
                  (:`NewEnumerator0`
                    (bind _state_4 (`self.AddDialogue` "Laura" "Utilise le et reviens me voir." (`|MakeArray` "Continuer" :!type "Text")))
                    (switch `/Game/SummerLearning/Blueprints/Dialogue/Enum_DialogueState` _state_4
                      (:`NewEnumerator0`
                        (`self.SetDialogueTreeIndex` 1)
                        (`self.CloseConversation`))))))))))
      (:`1`
        (bind _state_5 (`self.AddDialogue` "Laura" "Reviens me voir quand tu seras un rectangle." (`|MakeArray` "Partir" :!type "Text")))
        (switch `/Game/SummerLearning/Blueprints/Dialogue/Enum_DialogueState` _state_5
          (:`NewEnumerator0`
            (`self.SetDialogueTreeIndex` 1)
            (`self.CloseConversation`)))))
    (else
      (switch `int` (`self.DialogueTreeIndex2`)
        (:`0`
          (bind _state_6 (`self.AddDialogue` "Laura" "Bien ! Maintenant tu es un rectangle." (`|MakeArray` "Continuer" :!type "Text")))
          (switch `/Game/SummerLearning/Blueprints/Dialogue/Enum_DialogueState` _state_6
            (:`NewEnumerator0`
              (bind _state_7 (`self.AddDialogue` "Laura" "Le rectangle possède six faces rectangulaires dont tous les angles sont droits." (`|MakeArray` "Continuer" :!type "Text")))
              (switch `/Game/SummerLearning/Blueprints/Dialogue/Enum_DialogueState` _state_7
                (:`NewEnumerator0`
                  (bind _state_8 (`self.AddDialogue` "Laura" "Rejoins moi maintenant de l'autre côté du mur." (`|MakeArray` "Continuer" :!type "Text")))
                  (switch `/Game/SummerLearning/Blueprints/Dialogue/Enum_DialogueState` _state_8
                    (:`NewEnumerator0`
                      (set `self.DialogueTreeIndex2` 1)
                      (`self.ClearDialogueProgress`)
                      (`self.CloseConversation`))))))))
        (:`1`
          (bind _state_9 (`self.AddDialogue` "Laura" "Je t'attends de l'autre côté. A tout de suite !" (`|MakeArray` "Continuer" :!type "Text")))
          (switch `/Game/SummerLearning/Blueprints/Dialogue/Enum_DialogueState` _state_9
            (:`NewEnumerator0`
              (set `self.DialogueTreeIndex2` 1)
              (`self.ClearDialogueProgress`)
              (`self.CloseConversation`))))))))