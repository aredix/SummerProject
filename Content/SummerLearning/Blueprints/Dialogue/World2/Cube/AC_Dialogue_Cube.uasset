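; Dialogue component in which Laura, in French, teaches the player, now a cube, what cubes and squares are.
; Overrides Dialogue as a chain of AddDialogue nodes gated on Pass Through, with an optional square explanation that rejoins the main path.
; The ending advances the tree index, closes the conversation, destroys the Cube NPC, reveals the Rectangle NPC's mesh and lets the player pass through walls.
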(fn `Dialogue`
  (`parent.Dialogue`)
  (switch `int` (`self.DialogueTreeIndex`)
    (:`0`
      (bind _state (`self.AddDialogue` "Laura" "Super te voilà !" (`|MakeArray` "Continuer" :!type "Text")))
      (switch `/Game/SummerLearning/Blueprints/Dialogue/Enum_DialogueState` _state
        (:`NewEnumerator0`
          (bind _state_2 (`self.AddDialogue` "Laura" "Comme tu peux le voir, tu es un cube." (`|MakeArray` "Continuer" :!type "Text")))
          (switch `/Game/SummerLearning/Blueprints/Dialogue/Enum_DialogueState` _state_2
            (:`NewEnumerator0`
              (bind _state_3 (`self.AddDialogue` "Laura" "Un cube est un objet à six faces carrées égales dont tous les angles sont droits." (`|MakeArray` "Continuer" :!type "Text")))
              (switch `/Game/SummerLearning/Blueprints/Dialogue/Enum_DialogueState` _state_3
                (:`NewEnumerator0`
                  (bind (_state_4 _optionindex) (`self.AddDialogue` "Laura" "Ah mais j'y pense, sais tu ce qu'est qu'un carré ?" (`|MakeArray` "Oui" "Non" :!type "Text")))
                  (switch `/Game/SummerLearning/Blueprints/Dialogue/Enum_DialogueState` _state_4
                    (:`NewEnumerator0`
                      (switch `int` _optionindex
                        (:`0`
                          (bind _state_5 (`self.AddDialogue` "Laura" "D'accord. Comme tu peux le voir, le passage est bloqué." (`|MakeArray` "Continuer" :!type "Text")))
                          (switch `/Game/SummerLearning/Blueprints/Dialogue/Enum_DialogueState` _state_5
                            (:`NewEnumerator0`
                              _)))
                        (:`1`
                          (bind _state_6 (`self.AddDialogue` "Laura" "Ah, laisses moi t'expliquer." (`|MakeArray` "Continuer" :!type "Text")))
                          (switch `/Game/SummerLearning/Blueprints/Dialogue/Enum_DialogueState` _state_6
                            (:`NewEnumerator0`
                              (bind _state_7 (`self.AddDialogue` "Laura" "Un carré est une forme géométrique qui a quatre côtés droits et quatre angles droits, tous les côtés ont la même longueur." (`|MakeArray` "D'accord" :!type "Text")))
                              (switch `/Game/SummerLearning/Blueprints/Dialogue/Enum_DialogueState` _state_7
                                (:`NewEnumerator0`
                                  (bind _state_8 (`self.AddDialogue` "Laura" "Bon, comme tu peux le voir, le passage est bloqué." (`|MakeArray` "Continuer" :!type "Text")))
                                  (switch `/Game/SummerLearning/Blueprints/Dialogue/Enum_DialogueState` _state_8
                                    (:`NewEnumerator0`
                                      _))))))))
                      (bind _state_9 (`self.AddDialogue` "Laura" "Mais, comme tu peux le voir, il y a une forme dans le mur." (`|MakeArray` "Continuer" :!type "Text")))
                      (switch `/Game/SummerLearning/Blueprints/Dialogue/Enum_DialogueState` _state_9
                        (:`NewEnumerator0`
                          (bind _state_10 (`self.AddDialogue` "Laura" "Cette forme est comme la tienne !" (`|MakeArray` "Continuer" :!type "Text")))
                          (switch `/Game/SummerLearning/Blueprints/Dialogue/Enum_DialogueState` _state_10
                            (:`NewEnumerator0`
                              (bind _state_11 (`self.AddDialogue` "Laura" "Si tu sautes pour passer au travers, tu me rejoindras de l'autre côté ! Je t'y attends." (`|MakeArray` "Continuer" :!type "Text")))
                              (switch `/Game/SummerLearning/Blueprints/Dialogue/Enum_DialogueState` _state_11
                                (:`NewEnumerator0`
                                  (`self.SetDialogueTreeIndex` 1)
                                  (`self.CloseConversation`)
                                  (bind _returnvalue (`GameplayStatics.GetActorOfClass` "/Game/SummerLearning/Blueprints/Dialogue/World2/Cube/BP_NPC_Cube.BP_NPC_Cube_C"))
                                  (`Actor.K2_DestroyActor` _returnvalue)
                                  (bind _returnvalue_2 (`GameplayStatics.GetActorOfClass` "/Game/SummerLearning/Blueprints/Dialogue/World2/Rectangle/BP_NPC_Rectangle.BP_NPC_Rectangle_C"))
                                  (`SceneComponent.SetVisibility` (`Character.Mesh` _returnvalue_2) true false)
                                  (bind _asbp_base_player (cast `/Game/SummerLearning/Blueprints/Player/BP_BasePlayer` (`GameplayStatics.GetPlayerPawn` 0)))
                                  (set `/Game/SummerLearning/Blueprints/Player/BP_BasePlayer.CanPassThroughWalls` true _asbp_base_player))))))))))))))))))