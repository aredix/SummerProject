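; Color-change trigger that applies yellow to a BP_BasePlayer overlapping its ChangeColor component, following primary color mixing.
; A switch on the player's Color turns red to orange and blue to green, while yellow or any unlisted color becomes yellow.
; Each valid change updates both the Shape material and the Color variable.
; Secondary colors (violet, orange, green) are left unchanged and print an invalid-color message.
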(event `self.ChangeColor.OnComponentBeginOverlap`
  (params (OverlappedComponent :type "PrimitiveComponent Object Reference") (OtherActor :type "Actor Object Reference") (OtherComp :type "PrimitiveComponent Object Reference") (OtherBodyIndex :type Integer) (bFromSweep :type Boolean) (SweepResult :type "HitResult Structure (by ref)"))
  (bind _asbp_base_player (cast `/Game/SummerLearning/Blueprints/Player/BP_BasePlayer` OtherActor))
  (switch `/Game/SummerLearning/Blueprints/Player/PlayerColorStatus` (`/Game/SummerLearning/Blueprints/Player/BP_BasePlayer.Color` _asbp_base_player)
    (:`NewEnumerator6`
      (bind _shape (`/Game/SummerLearning/Blueprints/Player/BP_BasePlayer.Shape` _asbp_base_player))
      (`PrimitiveComponent.SetMaterial` _shape 0 "/Game/SummerLearning/Materials/Yellow.Yellow" :!label _label)
      (set `/Game/SummerLearning/Blueprints/Player/BP_BasePlayer.Color` "NewEnumerator1" _asbp_base_player))
    (:`NewEnumerator0`
      (`KismetSystemLibrary.PrintString` "Couleur invalide" :!label _label_2))
    (:`NewEnumerator1`
      (goto _label))
    (:`NewEnumerator2`
      (goto _label_2))
    (:`NewEnumerator3`
      (`PrimitiveComponent.SetMaterial` _shape 0 "/Game/SummerLearning/Materials/Orange.Orange")
      (set `/Game/SummerLearning/Blueprints/Player/BP_BasePlayer.Color` "NewEnumerator2" _asbp_base_player))
    (:`NewEnumerator4`
      (goto _label_2))
    (:`NewEnumerator5`
      (`PrimitiveComponent.SetMaterial` _shape 0 "/Game/SummerLearning/Materials/Green.Green")
      (set `/Game/SummerLearning/Blueprints/Player/BP_BasePlayer.Color` "NewEnumerator4" _asbp_base_player))))

(fn `UserConstructionScript`)