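; Dialogue component for World 3's yellow color lesson, where Laura, speaking French, sends the player to pick up a color modifier.
; An override of Dialogue branches on DialogueTreeIndex: the intro enables color changing, then later talks check the player's color.
; The correct color enables passing through walls, destroys BP_NPC_Jaune and reveals BP_NPC_Bleu's mesh; otherwise Laura asks again.
; Each branch increments its own dialogue counter on BP_BasePlayer.
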(fn `Dialogue`
  (`parent.Dialogue`)
  (bind _asbp_base_player (cast `/Game/SummerLearning/Blueprints/Player/BP_BasePlayer` (`GameplayStatics.GetPlayerPawn` 0)))
  (switch `int` (`self.DialogueTreeIndex`)
    (:`0`
      (`/Engine/EditorBlueprintResources/StandardMacros.IncrementInt` (`/Game/SummerLearning/Blueprints/Player/BP_BasePlayer.CompteurDialoguePrincipal` _asbp_base_player)
        (:`  `
          (bind _state (`self.AddDialogue` "Laura" "Passons maintenant à la couleur jaune." (`|MakeArray` "Continuer" :!type "Text")))
          (switch `/Game/SummerLearning/Blueprints/Dialogue/Enum_DialogueState` _state
            (:`NewEnumerator0`
              (bind _state_2 (`self.AddDialogue` "Laura" "La couleur jaune est la couleur du soleil ou encore, des bananes !" (`|MakeArray` "Continuer" :!type "Text")))
              (switch `/Game/SummerLearning/Blueprints/Dialogue/Enum_DialogueState` _state_2
                (:`NewEnumerator0`
                  (bind _state_3 (`self.AddDialogue` "Laura" "Derrière toi se trouve un modificateur qui va te permettre de prendre la couleur jaune." (`|MakeArray` "Continuer" :!type "Text")))
                  (switch `/Game/SummerLearning/Blueprints/Dialogue/Enum_DialogueState` _state_3
                    (:`NewEnumerator0`
                      (bind _state_4 (`self.AddDialogue` "Laura" "Prends-le et reviens voir une fois que c'est fait." (`|MakeArray` "Continuer" :!type "Text")))
                      (switch `/Game/SummerLearning/Blueprints/Dialogue/Enum_DialogueState` _state_4
                        (:`NewEnumerator0`
                          (`self.SetDialogueTreeIndex` 1)
                          (`self.CloseConversation`)
                          (set `/Game/SummerLearning/Blueprints/Player/BP_BasePlayer.CanChangeColor` true _asbp_base_player))))))))))))
    (:`1`
      (if (`|EnumEquality` (`/Game/SummerLearning/Blueprints/Player/BP_BasePlayer.Color` _asbp_base_player) "NewEnumerator1")
        (`/Engine/EditorBlueprintResources/StandardMacros.IncrementInt` (`/Game/SummerLearning/Blueprints/Player/BP_BasePlayer.CompteurDialogueSuite` _asbp_base_player)
          (:`  `
            (bind _state_5 (`self.AddDialogue` "Laura" "Super ! Maintenant tu peux passer au travers du mur." (`|MakeArray` "Continuer" :!type "Text")))
            (switch `/Game/SummerLearning/Blueprints/Dialogue/Enum_DialogueState` _state_5
              (:`NewEnumerator0`
                (`self.SetDialogueTreeIndex` 1)
                (`self.CloseConversation`)
                (bind _returnvalue (`GameplayStatics.GetActorOfClass` "/Game/SummerLearning/Blueprints/Dialogue/World3/Jaune/BP_NPC_Jaune.BP_NPC_Jaune_C"))
                (`Actor.K2_DestroyActor` _returnvalue)
                (bind _returnvalue_2 (`GameplayStatics.GetActorOfClass` "/Game/SummerLearning/Blueprints/Dialogue/World3/Bleu/BP_NPC_Bleu.BP_NPC_Bleu_C"))
                (`SceneComponent.SetVisibility` (`Character.Mesh` _returnvalue_2) true false)
                (set `/Game/SummerLearning/Blueprints/Player/BP_BasePlayer.CanPassThroughWalls` true _asbp_base_player)))))
        (else
          (`/Engine/EditorBlueprintResources/StandardMacros.IncrementInt` (`/Game/SummerLearning/Blueprints/Player/BP_BasePlayer.CompteurDialogueErreur` _asbp_base_player)
            (:`  `
              (bind _state_6 (`self.AddDialogue` "Laura" "Tu n'as pas encore changé de couleur. Reviens me voir une fois que c'est fait." (`|MakeArray` "Continuer" :!type "Text")))
              (switch `/Game/SummerLearning/Blueprints/Dialogue/Enum_DialogueState` _state_6
                (:`NewEnumerator0`
                  (`self.SetDialogueTreeIndex` 1)
                  (`self.CloseConversation`))))))))))