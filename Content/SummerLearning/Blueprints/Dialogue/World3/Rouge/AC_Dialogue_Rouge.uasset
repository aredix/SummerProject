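; Dialogue component for Laura in the World 3 red area, a French lesson introducing the three primary colours.
; The Dialogue override switches on DialogueTreeIndex: a chained intro explains red, blue and yellow, sends the player to grab a red colour modifier, then advances the index.
; Later talks check the player's Color to either allow passing through the wall or remind them to change colour.
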(fn `Dialogue`
  (`parent.Dialogue`)
  (bind _asbp_base_player (cast `/Game/SummerLearning/Blueprints/Player/BP_BasePlayer` (`GameplayStatics.GetPlayerPawn` 0)))
  (switch `int` (`self.DialogueTreeIndex`)
    (:`0`
      (bind _state (`self.AddDialogue` "Laura" "Bon, te voilà à présent dans le monde des couleurs." (`|MakeArray` "Continuer" :!type "Text")))
      (switch `/Game/SummerLearning/Blueprints/Dialogue/Enum_DialogueState` _state
        (:`NewEnumerator0`
          (bind _state_2 (`self.AddDialogue` "Laura" "Tout objet dans le monde a sa propre couleur et il en existe une infinité." (`|MakeArray` "Continuer" :!type "Text")))
          (switch `/Game/SummerLearning/Blueprints/Dialogue/Enum_DialogueState` _state_2
            (:`NewEnumerator0`
              (bind _state_3 (`self.AddDialogue` "Laura" "Rassures toi, on ne va pas toutes les apprendre. On va juste se concentrer sur les couleurs primaires. " (`|MakeArray` "Continuer" :!type "Text")))
              (switch `/Game/SummerLearning/Blueprints/Dialogue/Enum_DialogueState` _state_3
                (:`NewEnumerator0`
                  (bind _state_4 (`self.AddDialogue` "Laura" "Les couleurs primaires se compte au nombre de 3." (`|MakeArray` "Continuer" :!type "Text")))
                  (switch `/Game/SummerLearning/Blueprints/Dialogue/Enum_DialogueState` _state_4
                    (:`NewEnumerator0`
                      (bind _state_5 (`self.AddDialogue` "Laura" "Le rouge, qui est par exemple la couleur des fraises mais aussi des tomates." (`|MakeArray` "Continuer" :!type "Text")))
                      (switch `/Game/SummerLearning/Blueprints/Dialogue/Enum_DialogueState` _state_5
                        (:`NewEnumerator0`
                          (bind _state_6 (`self.AddDialogue` "Laura" "Le bleu, qui est la couleur du ciel en pleine journée mais aussi la couleur de l'océan." (`|MakeArray` "Continuer" :!type "Text")))
                          (switch `/Game/SummerLearning/Blueprints/Dialogue/Enum_DialogueState` _state_6
                            (:`NewEnumerator0`
                              (bind _state_7 (`self.AddDialogue` "Laura" "Et le jaune, qui est la couleur des bananes ou encore des tournesols !" (`|MakeArray` "Continuer" :!type "Text")))
                              (switch `/Game/SummerLearning/Blueprints/Dialogue/Enum_DialogueState` _state_7
                                (:`NewEnumerator0`
                                  (bind _state_8 (`self.AddDialogue` "Laura" "Derrière toi se trouve un modificateur qui va te permettre de prendre la couleur rouge. Prends le et reviens voir une fois que c'est fait." (`|MakeArray` "Continuer" :!type "Text")))
                                  (switch `/Game/SummerLearning/Blueprints/Dialogue/Enum_DialogueState` _state_8
                                    (:`NewEnumerator0`
                                      (`self.SetDialogueTreeIndex` 1)
                                      (`self.CloseConversation`))))))))))))))))))
    (:`1`
      (if (`|EnumEquality` (`/Game/SummerLearning/Blueprints/Player/BP_BasePlayer.Color` _asbp_base_player) "NewEnumerator3")
        (bind _state_9 (`self.AddDialogue` "Laura" "Super ! Maintenant tu peux passer au travers du mur." (`|MakeArray` "Continuer" :!type "Text")))
        (switch `/Game/SummerLearning/Blueprints/Dialogue/Enum_DialogueState` _state_9
          (:`NewEnumerator0`
            (`self.SetDialogueTreeIndex` 1)
            (`self.CloseConversation`)))
        (else
          (bind _state_10 (`self.AddDialogue` "Laura" "Tu n'as pas encore changé de couleur. reviens me voir une fois que c'est fait." (`|MakeArray` "Continuer" :!type "Text")))
          (switch `/Game/SummerLearning/Blueprints/Dialogue/Enum_DialogueState` _state_10
            (:`NewEnumerator0`
              (`self.SetDialogueTreeIndex` 1)
              (`self.CloseConversation`))))))))