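; Dialogue component for the spawn NPC in World 1, where Laura welcomes the player in French and introduces the look and move controls.
; It extends a parent dialogue, switching on the tree index to play chained lines that each offer a single option.
; The first branch advances the index and allows looking but not moving.
; The second enables movement, destroys BP_NPC_Spawn and makes the BP_NPC_Jump mesh visible.
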(fn `Dialogue`
  (`parent.Dialogue`)
  (switch `int` (`self.DialogueTreeIndex`)
    (:`0`
      (bind _state (`self.AddDialogue` "Inconnu" "Bienvenue ! J'espère que tu vas bien !" (`|MakeArray` "Continuer" :!type "Text")))
      (switch `/Game/SummerLearning/Blueprints/Dialogue/Enum_DialogueState` _state
        (:`NewEnumerator0`
          (bind _state_2 (`self.AddDialogue` "Laura" "Moi c'est Laura et aujourd'hui on va vivre une superbe aventure tous les deux." (`|MakeArray` "Continuer" :!type "Text")))
          (switch `/Game/SummerLearning/Blueprints/Dialogue/Enum_DialogueState` _state_2
            (:`NewEnumerator0`
              (bind _state_3 (`self.AddDialogue` "Laura" "Je vais te faire découvrir au travers de mon monde, les formes et les couleurs ! Tu vas voir c'est génial ! " (`|MakeArray` "Continuer" :!type "Text")))
              (switch `/Game/SummerLearning/Blueprints/Dialogue/Enum_DialogueState` _state_3
                (:`NewEnumerator0`
                  (bind _state_4 (`self.AddDialogue` "Laura" "Déjà dans un premier temps, je vais t'apprendre à te déplacer dans mon monde." (`|MakeArray` "Continuer" :!type "Text")))
                  (switch `/Game/SummerLearning/Blueprints/Dialogue/Enum_DialogueState` _state_4
                    (:`NewEnumerator0`
                      (bind _state_5 (`self.AddDialogue` "Laura" "Utilise ta souris pour regarder autour de toi !  Ensuite, reviens me voir." (`|MakeArray` "Regarder autour" :!type "Text")))
                      (switch `/Game/SummerLearning/Blueprints/Dialogue/Enum_DialogueState` _state_5
                        (:`NewEnumerator0`
                          (`self.SetDialogueTreeIndex` 1)
                          (`self.CloseConversation`)
                          (bind _asbp_base_player (cast `/Game/SummerLearning/Blueprints/Player/BP_BasePlayer` (`GameplayStatics.GetPlayerPawn` 0)))
                          (set `/Game/SummerLearning/Blueprints/Player/BP_BasePlayer.CanMove` false _asbp_base_player)
                          (set `/Game/SummerLearning/Blueprints/Player/BP_BasePlayer.CanLookAround` true _asbp_base_player))))))))))))
    (:`1`
      (bind _state_6 (`self.AddDialogue` "Laura" "Bien ! Maintenant, rejoins-moi un peu plus loin afin de pouvoir en apprendre plus ! " (`|MakeArray` "Continuer" :!type "Text")))
      (switch `/Game/SummerLearning/Blueprints/Dialogue/Enum_DialogueState` _state_6
        (:`NewEnumerator0`
          (bind _state_7 (`self.AddDialogue` "Laura" "Utilise les touches Z,Q,S et D pour te déplacer." (`|MakeArray` "Continuer" :!type "Text")))
          (switch `/Game/SummerLearning/Blueprints/Dialogue/Enum_DialogueState` _state_7
            (:`NewEnumerator0`
              (bind _asbp_base_player_2 (cast `/Game/SummerLearning/Blueprints/Player/BP_BasePlayer` (`GameplayStatics.GetPlayerPawn` 0)))
              (set `/Game/SummerLearning/Blueprints/Player/BP_BasePlayer.CanMove` true _asbp_base_player_2)
              (`self.CloseConversation`)
              (bind _returnvalue (`GameplayStatics.GetActorOfClass` "/Game/SummerLearning/Blueprints/Dialogue/Wolrd1/NPC_Spawn/BP_NPC_Spawn.BP_NPC_Spawn_C"))
              (`Actor.K2_DestroyActor` _returnvalue)
              (bind _returnvalue_2 (`GameplayStatics.GetActorOfClass` "/Game/SummerLearning/Blueprints/Dialogue/Wolrd1/NPC_Jump/BP_NPC_Jump.BP_NPC_Jump_C"))
              (`SceneComponent.SetVisibility` (`Character.Mesh` _returnvalue_2) true false))))))))