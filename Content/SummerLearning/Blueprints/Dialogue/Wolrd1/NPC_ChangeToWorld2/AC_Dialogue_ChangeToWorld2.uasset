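; Dialogue component for the world 1 NPC that sends the player on to world 2.
; It extends a parent dialogue and shows one French line from an unknown speaker with a single option to move to world 2.
; On pass-through it closes the conversation, opens the level named by its LevelName variable and prints that name.
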(fn `Dialogue`
  (bind _level_name (`self.Level Name`))
  (`parent.Dialogue`)
  (switch `int` (`self.DialogueTreeIndex`)
    (:`0`
      (bind _state (`self.AddDialogue` "Inconnu" "Super ! Aller on en a fini pour ici, allons au monde suivant !" (`|MakeArray` "Passer au monde 2" :!type "Text")))
      (switch `/Game/SummerLearning/Blueprints/Dialogue/Enum_DialogueState` _state
        (:`NewEnumerator0`
          (`self.CloseConversation`)
          (`GameplayStatics.OpenLevel` _level_name)
          (`KismetSystemLibrary.PrintString` (`KismetStringLibrary.Conv_NameToString` _level_name)))))))