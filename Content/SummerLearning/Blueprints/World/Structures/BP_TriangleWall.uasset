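; BP_TriangleWall is a wall that lets the player pass only in a specific status, likely the triangle form, optionally also requiring a matching color.
; Overlapping the CB_VerifTriangle trigger checks status and color, then disables CBPassageTriangle collision on success or keeps it solid otherwise.
; Leaving the CB_FinTriangle trigger restores the passage's collision.
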(event `self.CB_VerifTriangle.OnComponentBeginOverlap`
  (params (OverlappedComponent :type "PrimitiveComponent Object Reference") (OtherActor :type "Actor Object Reference") (OtherComp :type "PrimitiveComponent Object Reference") (OtherBodyIndex :type Integer) (bFromSweep :type Boolean) (SweepResult :type "HitResult Structure (by ref)"))
  (bind _cb_passagetriangle (`self.CB_PassageTriangle`))
  (bind _asbp_base_player (cast `/Game/SummerLearning/Blueprints/Player/BP_BasePlayer` OtherActor))
  (if (`|EnumEquality` (`/Game/SummerLearning/Blueprints/Player/BP_BasePlayer.Status` _asbp_base_player) "NewEnumerator2")
    (if (`self.isColorBased`)
      (if (`|EnumEquality` (`/Game/SummerLearning/Blueprints/Player/BP_BasePlayer.Color` _asbp_base_player) (`self.ColorRequired`))
        (`PrimitiveComponent.SetCollisionEnabled` _cb_passagetriangle "NoCollision" :!label _label)
        (else
          (`PrimitiveComponent.SetCollisionEnabled` _cb_passagetriangle "QueryAndPhysics" :!label _label_2)))
      (else
        (goto _label)))
    (else
      (goto _label_2))))

(event `self.CB_FinTriangle.OnComponentEndOverlap`
  (params (OverlappedComponent :type "PrimitiveComponent Object Reference") (OtherActor :type "Actor Object Reference") (OtherComp :type "PrimitiveComponent Object Reference") (OtherBodyIndex :type Integer))
  (cast `/Game/SummerLearning/Blueprints/Player/BP_BasePlayer` OtherActor)
  (`PrimitiveComponent.SetCollisionEnabled` (`self.CB_PassageTriangle`) "QueryAndPhysics"))

(fn `UserConstructionScript`)