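; Dialogue component for the World 2 riddle, where Laura tests whether the player can take the right shape to pass through a wall.
; The Dialogue override chains Continue-only lines on tree index 0, resetting the player's mesh to a cube before the last one.
; When the conversation ends it advances the index, destroys BP_NPC_Enigme, reveals the BP_NPC_ChangeToWorld3 mesh and enables the player's shape change and wall pass-through.
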(fn `Dialogue`
  (`parent.Dialogue`)
  (switch `int` (`self.DialogueTreeIndex`)
    (:`0`
      (bind _state (`self.AddDialogue` "Laura" "Bien. Maintenant, on va voir si tu as tout retenu." (`|MakeArray` "Continuer" :!type "Text")))
      (switch `/Game/SummerLearning/Blueprints/Dialogue/Enum_DialogueState` _state
        (:`NewEnumerator0`
          (bind _state_2 (`self.AddDialogue` "Laura" "Pour ce faire, tu vas devoir te rappeler de ce que je t'ai appris auparavant et prendre la bonne forme pour passer au travers de ce mur." (`|MakeArray` "Continuer" :!type "Text")))
          (switch `/Game/SummerLearning/Blueprints/Dialogue/Enum_DialogueState` _state_2
            (:`NewEnumerator0`
              (bind _state_3 (`self.AddDialogue` "Laura" "Mais avant tout, laisse moi te rendre ta forme originale." (`|MakeArray` "Continuer" :!type "Text")))
              (switch `/Game/SummerLearning/Blueprints/Dialogue/Enum_DialogueState` _state_3
                (:`NewEnumerator0`
                  (bind _asbp_base_player (cast `/Game/SummerLearning/Blueprints/Player/BP_BasePlayer` (`GameplayStatics.GetPlayerPawn` 0)))
                  (`StaticMeshComponent.SetStaticMesh` (`/Game/SummerLearning/Blueprints/Player/BP_BasePlayer.Shape` _asbp_base_player) "/Game/SummerLearning/Blueprints/Player/StaticMeshes/SM_PlayerCube.SM_PlayerCube")
                  (bind _state_4 (`self.AddDialogue` "Laura" "Bien. A toi de jouer." (`|MakeArray` "Continuer" :!type "Text")))
                  (switch `/Game/SummerLearning/Blueprints/Dialogue/Enum_DialogueState` _state_4
                    (:`NewEnumerator0`
                      (`self.SetDialogueTreeIndex` 1)
                      (`self.CloseConversation`)
                      (bind _returnvalue (`GameplayStatics.GetActorOfClass` "/Game/SummerLearning/Blueprints/Dialogue/World2/Enigme/BP_NPC_Enigme.BP_NPC_Enigme_C"))
                      (`Actor.K2_DestroyActor` _returnvalue)
                      (bind _returnvalue_2 (`GameplayStatics.GetActorOfClass` "/Game/SummerLearning/Blueprints/Dialogue/World2/ChangeToWorld3/BP_NPC_ChangeToWorld3.BP_NPC_ChangeToWorld3_C"))
                      (`SceneComponent.SetVisibility` (`Character.Mesh` _returnvalue_2) true false)
                      (set `/Game/SummerLearning/Blueprints/Player/BP_BasePlayer.CanChangeShape` true _asbp_base_player)
                      (set `/Game/SummerLearning/Blueprints/Player/BP_BasePlayer.CanPassThroughWalls` true _asbp_base_player))))))))))))