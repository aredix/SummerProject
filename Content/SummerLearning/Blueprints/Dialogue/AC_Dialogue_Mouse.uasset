(fn `Dialogue`
  (`parent.Dialogue`)
  (switch `int` (`self.DialogueTreeIndex`)
    (:`0`
      (bind (_state _optionindex) (`self.AddDialogue` "La souris" "Salut t'as du fromage mon reuf ?" (`|MakeArray` "Tiens mon reuf" "J'suis à sec pélo" :!type "Text")))
      (switch `/Game/SummerLearning/Blueprints/Dialogue/Enum_DialogueState` _state
        (:`NewEnumerator0`
          (switch `int` _optionindex
            (:`0`
              (bind (_state_2 _optionindex_2) (`self.AddDialogue` "La souris" "Super ! Je peux en avoir ?" (`|MakeArray` "Tiens !" "Nope désolé je garde pour moi" :!type "Text")))
              (switch `/Game/SummerLearning/Blueprints/Dialogue/Enum_DialogueState` _state_2
                (:`NewEnumerator0`
                  (switch `int` _optionindex_2
                    (:`0`
                      (bind _state_3 (`self.AddDialogue` "La souris" "Merci t'es un boss !" (`|MakeArray` "Pas de souci le sang !" :!type "Text")))
                      (switch `/Game/SummerLearning/Blueprints/Dialogue/Enum_DialogueState` _state_3
                        (:`NewEnumerator0`
                          (`self.SetDialogueTreeIndex` 1)
                          (`self.CloseConversation`))))
                    (:`1`
                      (bind _state_4 (`self.AddDialogue` "La souris" "Oh t'abuses ! " (`|MakeArray` "Aller cheh !!" :!type "Text")))
                      (switch `/Game/SummerLearning/Blueprints/Dialogue/Enum_DialogueState` _state_4
                        (:`NewEnumerator0`
                          (`self.ClearDialogueProgress`)
                          (`self.CloseConversation`))))))))
            (:`1`
              (bind _state_5 (`self.AddDialogue` "La souris" "Ah dommage ..." (`|MakeArray` "Aller j'y vais ! Bye bye !" :!type "Text")))
              (switch `/Game/SummerLearning/Blueprints/Dialogue/Enum_DialogueState` _state_5
                (:`NewEnumerator0`
                  (`self.ClearDialogueProgress`)
                  (`self.CloseConversation`))))))))
    (:`1`
      (bind _state_6 (`self.AddDialogue` "La souris" "Merci de m'avoir donné du frommage mon reuf ! Je m'en souviendrais !" (`|MakeArray` "Avec plaisir fraté" :!type "Text")))
      (switch `/Game/SummerLearning/Blueprints/Dialogue/Enum_DialogueState` _state_6
        (:`NewEnumerator0`
          (`self.ClearDialogueProgress`)
          (`self.CloseConversation`))))))