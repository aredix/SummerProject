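; BP_CubeWall is a wall that lets the player through only when their Status matches the first value of its enum.
; Entering the verification box checks the BP_BasePlayer Status and switches the passage cube's collision off on a match, or to query-and-physics otherwise.
; Leaving the separate end box restores the passage cube's collision, closing the wall again.
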(event `self.CB_VerificationCube.OnComponentBeginOverlap`
  (params (OverlappedComponent :type "PrimitiveComponent Object Reference") (OtherActor :type "Actor Object Reference") (OtherComp :type "PrimitiveComponent Object Reference") (OtherBodyIndex :type Integer) (bFromSweep :type Boolean) (SweepResult :type "HitResult Structure (by ref)"))
  (bind _cb_passagecube (`self.CB_PassageCube`))
  (bind _asbp_base_player (cast `/Game/SummerLearning/Blueprints/Player/BP_BasePlayer` OtherActor))
  (if (`|EnumEquality` (`/Game/SummerLearning/Blueprints/Player/BP_BasePlayer.Status` _asbp_base_player) "NewEnumerator0")
    (`PrimitiveComponent.SetCollisionEnabled` _cb_passagecube "NoCollision")
    (else
      (`PrimitiveComponent.SetCollisionEnabled` _cb_passagecube "QueryAndPhysics"))))

(event `self.CB_FinCube.OnComponentEndOverlap`
  (params (OverlappedComponent :type "PrimitiveComponent Object Reference") (OtherActor :type "Actor Object Reference") (OtherComp :type "PrimitiveComponent Object Reference") (OtherBodyIndex :type Integer))
  (cast `/Game/SummerLearning/Blueprints/Player/BP_BasePlayer` OtherActor)
  (`PrimitiveComponent.SetCollisionEnabled` (`self.CB_PassageCube`) "QueryAndPhysics"))

(fn `UserConstructionScript`)